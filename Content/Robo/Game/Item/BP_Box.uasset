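; BP_Box is an interactable box that is replaced by a holy item spline VFX actor when F is pressed nearby.
; A collision overlap with any Character toggles a prompt widget, which rotates every tick to face the player camera.
; PressF calls BoxCheck, which, only while the widget is visible, destroys the box and spawns BP_SplineVFX_HolyItem slightly offset from its location.
; ReleaseF does nothing.
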(event `self.ReceiveTick`
  (params (DeltaSeconds :type "Float (single-precision)"))
  (`SceneComponent.K2_SetWorldRotation` (`self.Widget`) (`KismetMathLibrary.FindLookAtRotation` (`SceneComponent.K2_GetComponentLocation` (`self.Widget`)) (`PlayerCameraManager.GetCameraLocation` (`GameplayStatics.GetPlayerCameraManager` 0))) false false))

(event `self.BoxCollision.OnComponentBeginOverlap`
  (params (OverlappedComponent :type "PrimitiveComponent Object Reference") (OtherActor :type "Actor Object Reference") (OtherComp :type "PrimitiveComponent Object Reference") (OtherBodyIndex :type Integer) (bFromSweep :type Boolean) (SweepResult :type "HitResult Structure (by ref)"))
  (cast `Character` OtherActor)
  (`SceneComponent.SetVisibility` (`self.Widget`) true false)
  (set `self.IsWidgetVisible` true))

(event `self.BoxCollision.OnComponentEndOverlap`
  (params (OverlappedComponent :type "PrimitiveComponent Object Reference") (OtherActor :type "Actor Object Reference") (OtherComp :type "PrimitiveComponent Object Reference") (OtherBodyIndex :type Integer))
  (cast `Character` OtherActor)
  (`SceneComponent.SetVisibility` (`self.Widget`) false false)
  (set `self.IsWidgetVisible` false))

(event `BoxCheck`
  (if (`self.IsWidgetVisible`)
    (bind _output_get (set `self.BoxLocation` (`self.K2_GetActorLocation`)))
    (`self.K2_DestroyActor`)
    (`|SpawnActorFromClass` "/Game/Robo/Game/Item/BP_SplineVFX_HolyItem.BP_SplineVFX_HolyItem_C" (`KismetMathLibrary.MakeTransform` (`KismetMathLibrary.MakeVector` (+ (.x _output_get) -100.0) (.y _output_get) (.z _output_get)) (struct :`Yaw` 90.0) (0.5 0.5 0.5)) "Undefined" "MultiplyWithRoot" null null)))

(fn `PressF`
  (params (NewParam :type "Character Object Reference"))
  (returns (NewParam1 :type Boolean))
  (`self.BoxCheck`)
  (return false))

(fn `ReleaseF`
  (params (NewParam :type Boolean))
  (returns (NewParam1 :type Boolean))
  (return false))

(fn `UserConstructionScript`)